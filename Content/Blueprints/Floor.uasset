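; Floor actor that can display a targeting reticule component under the player's mouse cursor.
; PaintReticule either hides the Reticule or shows it and moves it to the cursor's hit location, using a complex trace on the Visibility channel.
; SetReticuleVisibility wraps the component's visibility toggle.
; The event graph and construction script are empty, so this Blueprint never calls PaintReticule itself.
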(fn `PaintReticule`
  (params (ShowReticule :type Boolean))
  (if ShowReticule
    (`self.SetReticuleVisibility` true)
    (`SceneComponent.K2_SetWorldLocation` (`self.Reticule`) (`.Location` (`GameplayStatics.BreakHitResult` (`PlayerController.GetHitResultUnderCursorByChannel` (`GameplayStatics.GetPlayerController` 0) "TraceTypeQuery1" true))) false false)
    (else
      (`self.SetReticuleVisibility` false))))

(fn `SetReticuleVisibility`
  (params (IsVisible :type Boolean))
  (`SceneComponent.SetVisibility` (`self.Reticule`) IsVisible false))

(fn `UserConstructionScript`)