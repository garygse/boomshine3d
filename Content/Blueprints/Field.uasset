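; Short-lived field actor that animates its mesh scale through a timeline on spawn, then destroys itself.
; It reports to the first Level actor found in the construction script, raising the active field count at start and lowering it when the timeline finishes.
; SetBaseColour keeps only the hue of the given colour, at full saturation and brightness, for both colour inputs of a dynamic material instance.
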(event `self.ReceiveBeginPlay`
  ;[1 1 1] Increase Active Field Count
  (`/Game/Blueprints/Level.AdjustActiveFields` (`self.Level`) 1)
  ;[1 1 1] Expand/Collapse Field Animation
  (bind (_direction _scale) (`Timeline|FieldTimeline`)
    (:`Update`
      (`SceneComponent.SetRelativeScale3D` (`self.StaticMeshComponent`) _scale))
    (:`Finished`
      (`self.K2_DestroyActor`)
      ;[1 1 1] Decrease Active Field Count
      (`/Game/Blueprints/Level.AdjustActiveFields` (`self.Level`) -1))))

(fn `SetBaseColour`
  (params (Colour :type "Vector Structure"))
  (bind _returnvalue (`KismetMathLibrary.HSVToRGB` (`KismetMathLibrary.RGBToHSV` (`KismetMathLibrary.Conv_VectorToLinearColor` Colour)) 1.0 1.0 1.0))
  (bind _returnvalue_2 (`PrimitiveComponent.CreateDynamicMaterialInstance` (`self.StaticMeshComponent`) 0 "/Game/DynamicRadial/MICs/MIC_Health_StyleA.MIC_Health_StyleA"))
  (`MaterialInstanceDynamic.SetVectorParameterValue` _returnvalue_2 "Color_InputA" _returnvalue)
  (`MaterialInstanceDynamic.SetVectorParameterValue` _returnvalue_2 "Color_InputB" _returnvalue))

(fn `UserConstructionScript`
  ;[1 1 1] Obtain Access to Level Variables
  (bind _outactors (`GameplayStatics.GetAllActorsOfClass` "/Game/Blueprints/Level.Level_C"))
  (set `self.Level` (`KismetArrayLibrary.Array_Get` _outactors)))